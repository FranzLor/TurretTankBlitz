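; Player controller for Turret Tank Blitz that toggles the pause menu on the Pause input action.
; A FlipFlop alternates between creating a new WBP_PauseMenu while pausing the game with a visible cursor and Game and UI input, and removing that menu while restoring game-only input and unpausing.
; The toggle state lives only in the FlipFlop, with no check of the actual pause state.
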(event `InputAction|Pause`
  (params (Key :type "Key Structure"))
  (bind _returnvalue (`GameplayStatics.GetPlayerController` 0))
  (bind _returnvalue_2 (`GameplayStatics.GetPlayerController` 0))
  (:`Pressed`
    (`/Engine/EditorBlueprintResources/StandardMacros.FlipFlop`
      (:`A`
        (bind _returnvalue_3 (`|CreateWidget` "/Game/Dynamic/Blueprints/Widgets/WBP_PauseMenu.WBP_PauseMenu_C"))
        (`UserWidget.AddToViewport` _returnvalue_3 0)
        (`GameplayStatics.SetGamePaused` true)
        (`WidgetBlueprintLibrary.SetInputMode_GameAndUIEx` _returnvalue_2 null)
        (set `PlayerController.bShowMouseCursor` true _returnvalue_2))
      (:`B`
        (`Widget.RemoveFromParent` _returnvalue_3)
        (`WidgetBlueprintLibrary.SetInputMode_GameOnly` _returnvalue)
        (set `PlayerController.bShowMouseCursor` false _returnvalue)
        (`GameplayStatics.SetGamePaused` false)))))

(fn `UserConstructionScript`)